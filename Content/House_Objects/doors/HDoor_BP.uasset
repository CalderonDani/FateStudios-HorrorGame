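; House door Blueprint that the player swings open and closed with the Interact key.
; A box trigger shows an InteractionPrompt widget and opens a Gate while MainCharacter_bp overlaps it, then removes the prompt and closes the Gate on exit.
; Interact presses passing the Gate flip-flop a timeline forward or backward, lerping the door mesh's yaw between closed and open.
; Each press also briefly flags the prompt as pressed, outside the Gate.
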(event OnComponentBeginOverlap(Box)
  (params (OverlappedComponent :type Primitive%20Component%20Object%20Reference) (OtherActor :type Actor%20Object%20Reference) (OtherComp :type Primitive%20Component%20Object%20Reference) (OtherBodyIndex :type Integer) (bFromSweep :type Boolean) (SweepResult :type Hit%20Result%20Structure%20%28by%20ref%29))
  (Utilities|Casting|CastToMainCharacter_bp OtherActor)
  (bind _returnvalue (UserInterface|CreateWidget "/Game/Menus/InteractionPrompt.InteractionPrompt_C"))
  (UserInterface|Viewport|AddtoViewport _returnvalue 0)
  (Utilities|FlowControl|Gate true) ; enters at Open
)

(event OnComponentEndOverlap(Box)
  (params (OverlappedComponent :type Primitive%20Component%20Object%20Reference) (OtherActor :type Actor%20Object%20Reference) (OtherComp :type Primitive%20Component%20Object%20Reference) (OtherBodyIndex :type Integer))
  (Utilities|Casting|CastToMainCharacter_bp OtherActor)
  (Widget|RemovefromParent (stale OnComponentBeginOverlap(Box) _returnvalue))
  (Utilities|FlowControl|Gate true) ; enters at Close
)

(event EventBeginPlay
  ;[1 1 1] Enable Interact Key
  (Input|EnableInput (Game|GetPlayerController 0)))

(event Input|ActionEvents|InputActionInteract
  (params (Key :type Key%20Structure :default "None"))
  (:Pressed
    (Variables|/Game/Menus/InteractionPrompt.InteractionPrompt_C|SetIsPressed (stale OnComponentBeginOverlap(Box) _returnvalue) true)
    (Utilities|FlowControl|Sequence
      (:then_0
        (Utilities|FlowControl|Gate true
          (:Exit
            (Utilities|FlowControl|FlipFlop
              (:A
                (bind _door_track (Timeline|Timeline_0 Play)
                  (:Update
                    (Transformation|SetRelativeRotation (Variables|Default|GetSM_WoodDoorStatic) (Math|Rotator|MakeRotator 90.000244 0.0 (Math|Float|Lerp (Variables|Default|GetClosedDoor) (Variables|Default|GetOpenDoor) _door_track)) false false))))
              (:B
                (Timeline|Timeline_0 Reverse))))))
      (:then_1
        (Utilities|FlowControl|Delay 0.2)
        (Variables|/Game/Menus/InteractionPrompt.InteractionPrompt_C|SetIsPressed (stale OnComponentBeginOverlap(Box) _returnvalue) false)))))

(fn ConstructionScript)